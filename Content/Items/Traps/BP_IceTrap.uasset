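; BP_IceTrap is a trap Blueprint that temporarily freezes the player it affects.
; Its TrapEffect event lowers walking braking deceleration, disables player input and calls FreezeCharacter on the player.
; After a retriggerable delay of EffectDuration, it restores input and braking, unfreezes the character and resets max speed to walking pace, a fix for players who entered while running.
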(event `self.TrapEffect`
  (params (Player :type "LeosCVCharacter Object Reference"))
  (bind _charactermovement (`Character.CharacterMovement` Player))
  ;[1 1 1] If freeze is added freeze the player input
  (set `CharacterMovementComponent.BrakingDecelerationWalking` 500.0 _charactermovement)
  (`self.DisableInput` Player null)
  (`LeosCVCharacter.FreezeCharacter` Player true)
  (`KismetSystemLibrary.RetriggerableDelay` (`self.EffectDuration`))
  (`self.EnableInput` Player null)
  (set `CharacterMovementComponent.BrakingDecelerationWalking` 2000.0 _charactermovement)
  (`LeosCVCharacter.FreezeCharacter` Player false)
  ;[1 1 1] Bug Fix: return to walk state in case you where running before enter
  (set `CharacterMovementComponent.MaxWalkSpeed` 150.0 _charactermovement))

(fn `UserConstructionScript`
  (`parent.UserConstructionScript`))